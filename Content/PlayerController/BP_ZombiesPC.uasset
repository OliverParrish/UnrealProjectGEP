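; BP_ZombiesPC is the player controller for a zombies game, handling the pause and end-of-match menus.
; Pressing Pause pauses the game and opens BP_PauseMenu, while HandleMatchFinished shows BP_WinMenu and OnCharDied shows BP_GameOverMenu, both stored as GameOverMenu.
; Each handler adds its widget to the viewport, switches player 0 to UI-only input and shows the mouse cursor.
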(event `InputAction|Pause`
  (params (Key :type "Key Structure"))
  (bind _returnvalue (`GameplayStatics.GetPlayerController` 0))
  (:`Pressed`
    (`GameplayStatics.SetGamePaused` true)
    (bind _returnvalue_2 (`|CreateWidget` "/Game/UI/BP_PauseMenu.BP_PauseMenu_C"))
    (bind _output_get (set `self.PauseMenu` _returnvalue_2))
    (`UserWidget.AddToViewport` _output_get 0)
    (`WidgetBlueprintLibrary.SetInputMode_UIOnlyEx` _returnvalue null)
    (set `PlayerController.bShowMouseCursor` true _returnvalue)))

(event `self.Handle_MatchFinished`
  (bind _returnvalue (`GameplayStatics.GetPlayerController` 0))
  (bind _returnvalue_2 (`|CreateWidget` "/Game/UI/BP_WinMenu.BP_WinMenu_C"))
  (bind _output_get (set `self.GameOverMenu` _returnvalue_2))
  (`UserWidget.AddToViewport` _output_get 0)
  (`WidgetBlueprintLibrary.SetInputMode_UIOnlyEx` _returnvalue null)
  (set `PlayerController.bShowMouseCursor` true _returnvalue))

(event `self.OnCharDied`
  (params (Char :type "ZombiesPChar Object Reference"))
  (bind _returnvalue (`GameplayStatics.GetPlayerController` 0))
  (bind _returnvalue_2 (`|CreateWidget` "/Game/UI/BP_GameOverMenu.BP_GameOverMenu_C"))
  (bind _output_get (set `self.GameOverMenu` _returnvalue_2))
  (`UserWidget.AddToViewport` _output_get 0)
  (`WidgetBlueprintLibrary.SetInputMode_UIOnlyEx` _returnvalue null)
  (set `PlayerController.bShowMouseCursor` true _returnvalue))

(fn `UserConstructionScript`)