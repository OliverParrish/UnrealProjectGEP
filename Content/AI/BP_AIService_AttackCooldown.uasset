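; Behavior tree service that re-enables an AI's ability to attack once its cooldown has elapsed.
; On each AI tick, while the can-attack Blackboard flag is false, it compares game time against the last attack time plus the cooldown, both read from Blackboard keys.
; It only sets the flag to true; clearing it and recording the attack time happen outside this service.
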(event `self.ReceiveTickAI`
  (params (OwnerController :type "AIController Object Reference") (ControlledPawn :type "Pawn Object Reference") (DeltaSeconds :type "Float (single-precision)"))
  (if (`BTFunctionLibrary.GetBlackboardValueAsBool` (`self.CanAttackKey`))
    _
    (elif (> (`KismetSystemLibrary.GetGameTimeInSeconds`) (+ (`BTFunctionLibrary.GetBlackboardValueAsFloat` (`self.LastAttackTimeKey`)) (`BTFunctionLibrary.GetBlackboardValueAsFloat` (`self.AttackCooldownKey`))))
      (`BTFunctionLibrary.SetBlackboardValueAsBool` (`self.CanAttackKey`) true))))